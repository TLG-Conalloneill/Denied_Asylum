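; Door Blueprint for a motion-controller grabbable door with a keyhole lock, with the door movement itself left unimplemented.
; Grab stores the controller as Hand when it is within the handle's collision sphere radius, and Release clears it if it matches.
; Tick sets Locked only while the keyhole is not unlocked and the door's yaw is near zero.
; The unlocked, held-hand branch is empty, and a look-at rotation toward the door is unused.
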(event EventGrab
  (params (MotionController :type Motion%20Controller%20Component%20Object%20Reference))
  (bind _handle_collision (Variables|Default|GetHandle%20Collision))
  (if (Utilities|Operators|EqualEqual (Transformation|GetWorldLocation MotionController) (Transformation|GetWorldLocation _handle_collision) (Variables|/Script/Engine.SphereComponent|GetSphereRadius _handle_collision))
    (Variables|Default|SetHand MotionController)))

(event EventRelease
  (params (MotionController :type Motion%20Controller%20Component%20Object%20Reference))
  (if (== MotionController (Variables|Default|GetHand))
    (Variables|Default|SetHand 0)))

(event EventTick
  (params (DeltaSeconds :type Float%20%28single-precision%29))
  (Utilities|FlowControl|Sequence
    (:then_0
      ;[1 1 1] Locked?
      (if (and (not (Variables|/Game/Conall_Denied_Asylum/DoorThings/Keyhole.Keyhole_C|GetUnlocked (Variables|Default|GetKeyHole))) (Math|Float|NearlyEqual(Float) (.yaw (Transformation|GetWorldRotation (Variables|Default|GetDoor_SM))) 0.0 1e-06))
        (Variables|Default|SetLocked true)
        (else
          (Variables|Default|SetLocked false))))
    (:then_1
      (if (not (Variables|Default|GetLocked))
        (Utilities|IsValid (Variables|Default|GetHand))))))

(fn ConstructionScript)